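; Moving cube hazard that bobs vertically and sends the player ball back to its recovery point on contact.
; Tick offsets the Cube by a move vector, which starts upward and flips direction when the Cube overlaps the LowLimit or HighLimit trigger.
; A Box overlap with the player pawn casts it to BallFallDownBall and teleports it to its RecoverLocation.
; Movement is a fixed per-frame step without delta time or sweep.
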(event `self.LowLimit.OnComponentBeginOverlap`
  (params (OverlappedComponent :type "PrimitiveComponent Object Reference") (OtherActor :type "Actor Object Reference") (OtherComp :type "PrimitiveComponent Object Reference") (OtherBodyIndex :type Integer) (bFromSweep :type Boolean) (SweepResult :type "HitResult Structure (by ref)"))
  (if (== OtherComp (`self.Cube`))
    (set `self.move vec` (0.0 0.0 1.0))))

(event `self.ReceiveBeginPlay`
  (set `self.move vec` (0.0 0.0 1.0)))

(event `self.HighLimit.OnComponentBeginOverlap`
  (params (OverlappedComponent :type "PrimitiveComponent Object Reference") (OtherActor :type "Actor Object Reference") (OtherComp :type "PrimitiveComponent Object Reference") (OtherBodyIndex :type Integer) (bFromSweep :type Boolean) (SweepResult :type "HitResult Structure (by ref)"))
  (if (== OtherComp (`self.Cube`))
    (set `self.move vec` (0.0 0.0 -1.0))))

(event `self.ReceiveTick`
  (params (DeltaSeconds :type "Float (single-precision)"))
  (`SceneComponent.K2_AddWorldOffset` (`self.Cube`) (`self.move vec`) false false))

(event `self.Box.OnComponentBeginOverlap`
  (params (OverlappedComponent :type "PrimitiveComponent Object Reference") (OtherActor :type "Actor Object Reference") (OtherComp :type "PrimitiveComponent Object Reference") (OtherBodyIndex :type Integer) (bFromSweep :type Boolean) (SweepResult :type "HitResult Structure (by ref)"))
  (bind _returnvalue (`GameplayStatics.GetPlayerPawn` 0))
  (if (== OtherActor _returnvalue)
    (bind _asball_fall_down_ball (cast `BallFallDownBall` _returnvalue))
    (`self.K2_SetActorLocation` _asball_fall_down_ball (`BallFallDownBall.RecoverLocation` _asball_fall_down_ball) false false)))

(fn `UserConstructionScript`)