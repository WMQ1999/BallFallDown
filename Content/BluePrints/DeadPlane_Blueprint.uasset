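; DeadPlane is a kill volume for the BallFallDown ball game that respawns the player when it falls into it.
; When the player pawn overlaps its Box, it casts it to BallFallDownBall and moves it to that ball's stored RecoverLocation.
; It also zeroes rotation and the Ball body's linear and angular physics velocity, then increments the ball's DeadTimes counter.
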(event `self.Box.OnComponentBeginOverlap`
  (params (OverlappedComponent :type "PrimitiveComponent Object Reference") (OtherActor :type "Actor Object Reference") (OtherComp :type "PrimitiveComponent Object Reference") (OtherBodyIndex :type Integer) (bFromSweep :type Boolean) (SweepResult :type "HitResult Structure (by ref)"))
  (bind _returnvalue (`GameplayStatics.GetPlayerPawn` 0))
  (if (== _returnvalue OtherActor)
    (bind _asball_fall_down_ball (cast `BallFallDownBall` _returnvalue))
    (`self.K2_SetActorLocation` _asball_fall_down_ball (`BallFallDownBall.RecoverLocation` _asball_fall_down_ball) false (`self.false`))
    (`self.K2_SetActorRotation` :`self` _asball_fall_down_ball :`bTeleportPhysics` (`self.false`))
    (bind _ball (`BallFallDownBall.Ball` _asball_fall_down_ball))
    (`PrimitiveComponent.SetPhysicsLinearVelocity` _ball (0.0 0.0 0.0) false "None")
    (`PrimitiveComponent.SetPhysicsAngularVelocityInDegrees` _ball (0.0 0.0 0.0) false "None")
    (set `BallFallDownBall.DeadTimes` (+ (`BallFallDownBall.DeadTimes` _asball_fall_down_ball) 1) _asball_fall_down_ball)))

(fn `UserConstructionScript`)